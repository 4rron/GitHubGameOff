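; BP_TrainingDummy is a damageable target actor in the interaction system that the player can kill.
; On any damage it subtracts the amount from Health and prints the remaining value.
; When Health reaches zero it calls KillCheck on the player's BP_InteractCharacter, passing its own class, then destroys itself.
; A failed character cast leaves the dummy alive.
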(event Game|Damage|EventAnyDamage
  (params (Damage :type Float%20%28single-precision%29) (DamageType :type Damage%20Type%20Object%20Reference) (InstigatedBy :type Controller%20Object%20Reference) (DamageCauser :type Actor%20Object%20Reference))
  (bind _output_get (Variables|Default|SetHealth (- (Variables|Default|GetHealth) Damage)))
  (Development|PrintString (Utilities|String|Append "Enemy health: " (Utilities|String|ToString(Float) _output_get)))
  (if (<= _output_get 0.0)
    (bind _asbp_interact_character (Utilities|Casting|CastToBP_InteractCharacter (Game|GetPlayerCharacter 0)))
    (Default|KillCheck _asbp_interact_character "BP_TrainingDummy_C")
    (Actor|DestroyActor)))

(fn ConstructionScript)